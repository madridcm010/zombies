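; Bullet actor for a top-down zombie shooter that kills any BP_ZombieAI its Sphere1 collision overlaps.
; On begin overlap it starts the death animation, zeroes walk speed and destroys the zombie immediately, with no delay for the animation.
; End overlap, unfiltered by actor type, decrements EnemiesAlive on BP_TopDownGameMode and calls CheckRemainingEnemies.
; The graph contains no movement or self-destruction logic for the bullet.
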(event `self.Sphere1.OnComponentBeginOverlap`
  (params (OverlappedComponent :type "PrimitiveComponent Object Reference") (OtherActor :type "Actor Object Reference") (OtherComp :type "PrimitiveComponent Object Reference") (OtherBodyIndex :type Integer) (bFromSweep :type Boolean) (SweepResult :type "HitResult Structure (by ref)"))
  (bind _asbp_zombie_ai (cast `/Game/TopDown/Blueprints/BP_ZombieAI` OtherActor))
  (`SkeletalMeshComponent.PlayAnimation` (`Character.Mesh` _asbp_zombie_ai) "/Game/TopDown/Animations/Zombie_Death.Zombie_Death" false)
  (set `CharacterMovementComponent.MaxWalkSpeed` 0.0 (`Character.CharacterMovement` _asbp_zombie_ai))
  (`self.K2_DestroyActor` _asbp_zombie_ai))

(event `self.Sphere1.OnComponentEndOverlap`
  (params (OverlappedComponent :type "PrimitiveComponent Object Reference") (OtherActor :type "Actor Object Reference") (OtherComp :type "PrimitiveComponent Object Reference") (OtherBodyIndex :type Integer))
  (bind _asbp_top_down_game_mode (cast `/Game/TopDown/Blueprints/BP_TopDownGameMode` (`GameplayStatics.GetGameMode`)))
  (`/Engine/EditorBlueprintResources/StandardMacros.DecrementInt` (`/Game/TopDown/Blueprints/BP_TopDownGameMode.Enemies_Alive` _asbp_top_down_game_mode)
    (:`  `
      (`/Game/TopDown/Blueprints/BP_TopDownGameMode.Check_Remaining_Enemies` _asbp_top_down_game_mode))))

(fn `UserConstructionScript`)