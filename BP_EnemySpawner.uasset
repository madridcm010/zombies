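; BP_EnemySpawner spawns zombie AI at its own transform in waves for the top-down game mode.
; On BeginPlay it binds Spawn_Enemy to the game mode's RespawnEnemy event.
; Each wave checks the alive-enemy cap per spawn, falling back to a delayed self-retrying event when full.
; Wave size grows by an increasing increment after each call.
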(event `self.ReceiveBeginPlay`
  (`|ExecutionSequence`
    (:`then_0`
      (bind _asbp_top_down_game_mode (cast `/Game/TopDown/Blueprints/BP_TopDownGameMode` (`GameplayStatics.GetGameMode`)))
      (set `self.As BP Top Down Game Mode` _asbp_top_down_game_mode)
      (add `/Game/TopDown/Blueprints/BP_TopDownGameMode.Respawn_Enemy` _asbp_top_down_game_mode (delegate `Spawn_Enemy`)))))

(event `Spawn_Enemy`
  (bind _as_bp_top_down_game_mode (`self.As BP Top Down Game Mode`))
  (for _ (range (`self.EnemySpawned`))
    (if (< (`/Game/TopDown/Blueprints/BP_TopDownGameMode.Enemies_Alive` _as_bp_top_down_game_mode) (`/Game/TopDown/Blueprints/BP_TopDownGameMode.Max_Enemies` _as_bp_top_down_game_mode))
      (`|SpawnActorFromClass` "/Game/TopDown/Blueprints/BP_ZombieAI.BP_ZombieAI_C" (`self.GetTransform`) "AdjustIfPossibleButAlwaysSpawn" "MultiplyWithRoot" null null)
      (else
        (`self.Spawn?`))))
  (`/Engine/EditorBlueprintResources/StandardMacros.IncrementInt` (`self.Spawn_Increment`)
    (:`  `
      (set `self.EnemySpawned` (+ (`self.EnemySpawned`) (`self.Spawn_Increment`))))))

(event `Spawn?`
  (bind _as_bp_top_down_game_mode (`self.As BP Top Down Game Mode`))
  (`KismetSystemLibrary.Delay` 1.2)
  (if (< (`/Game/TopDown/Blueprints/BP_TopDownGameMode.Enemies_Alive` _as_bp_top_down_game_mode) (`/Game/TopDown/Blueprints/BP_TopDownGameMode.Max_Enemies` _as_bp_top_down_game_mode))
    (`|SpawnActorFromClass` "/Game/TopDown/Blueprints/BP_ZombieAI.BP_ZombieAI_C" (`self.GetTransform`) "AdjustIfPossibleButAlwaysSpawn" "MultiplyWithRoot" null null)
    (else
      (`self.Spawn?`))))

(fn `UserConstructionScript`)